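; Game mode that runs Conway's Game of Life on a wrapping grid of BP_Tile actors.
; BeginPlay spawns the centred board with randomly active tiles, tracked in flattened tile and status arrays.
; While DoLoop is set, Tick applies birth and death rules in place on BoardStatusAux, so later tiles see earlier changes.
; The neighbour count checks the -X side twice and omits the +X,-Y diagonal, and the trailing Delay gates nothing.
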(event EventBeginPlay
  (CallFunction|SpawnBoard))

(event EventTick
  (params (DeltaSeconds :type Float%20%28single-precision%29))
  (if (Variables|Default|GetbDoLoop)
    (Variables|Default|SetBoardStatusAux (Variables|Default|GetBoardStatus))
    (for _index (range 0 (- (Variables|Default|GetBoardNX) 1))
      (for _index_2 (range 0 (- (Variables|Default|GetBoardNY) 1))
        (CallFunction|ProcessTile _index _index_2)))
    (Variables|Default|SetBoardStatus (Variables|Default|GetBoardStatusAux))
    (Utilities|FlowControl|Delay 0.2)))

(fn ConstructionScript)

(fn SpawnBoard
  (CallFunction|InitializeTiles)
  (LocalVariables|SetLNXHalf (Math|Float|Floor (/ (Math|Conversions|ToFloat(Integer) (Variables|Default|GetBoardNX)) 2.0)))
  (LocalVariables|SetLNYHalf (Math|Float|Floor (/ (Math|Conversions|ToFloat(Integer) (Variables|Default|GetBoardNY)) 2.0)))
  (for _index (range 0 (- (Variables|Default|GetBoardNX) 1))
    (LocalVariables|SetLX _index)
    (for _index_2 (range 0 (- (Variables|Default|GetBoardNY) 1))
      (LocalVariables|SetLY _index_2)
      (bind _output_get (LocalVariables|SetLOrigin (Math|Vector|MakeVector (* (- (LocalVariables|GetLX) (LocalVariables|GetLNXHalf)) (Variables|Default|GetTileLengthX)) (* (- (LocalVariables|GetLY) (LocalVariables|GetLNYHalf)) (Variables|Default|GetTileLengthY)) 0.0)))
      (bind _returnvalue (Game|SpawnActorfromClass "/Game/Framework/BP_Tile.BP_Tile_C" (Math|Transform|MakeTransform _output_get) "AlwaysSpawn" 0 0))
      (Utilities|FlowControl|Sequence
        (:then_0
          (CallFunction|AddTile (LocalVariables|GetLX) (LocalVariables|GetLY) _returnvalue))
        (:then_1
          (CallFunction|InitializeTile _returnvalue (LocalVariables|GetLX) (LocalVariables|GetLY)))))))

(fn AddTile
  (params (TileX :type Integer) (TileY :type Integer) (Tile :type BP%20Tile%20Object%20Reference))
  (Utilities|Array|SetArrayElem (Variables|Default|GetTiles) (CallFunction|GetTilePositioninArray TileX TileY) Tile))

(fn GetTilePositioninArray
  (params (X :type Integer) (Y :type Integer))
  (return (+ (* X (Variables|Default|GetBoardNX)) Y)))

(fn GetTile
  (params (TileX :type Integer) (TileY :type Integer))
  (return (Utilities|Array|Get(acopy) (Variables|Default|GetTiles) (CallFunction|GetTilePositioninArray TileX TileY))))

(fn InitializeTiles
  (CallFunction|InitializeStatus)
  (for _index (range 1 (* (Variables|Default|GetBoardNX) (Variables|Default|GetBoardNY)))
    (Utilities|Array|Add (Variables|Default|GetTiles) 0)))

(fn InitializeTile
  (params (InputPin :type BP%20Tile%20Object%20Reference) (TileX :type Integer) (TileY :type Integer))
  (bind _index (CallFunction|GetTilePositioninArray TileX TileY))
  (if (< (Math|Random|RandomFloat) (Variables|Default|GetInitialActivationProbability))
    (Default|Activate InputPin)
    (Utilities|Array|SetArrayElem (Variables|Default|GetBoardStatus) _index true)
    (else
      (Default|Deactivate InputPin)
      (Utilities|Array|SetArrayElem (Variables|Default|GetBoardStatus) _index false))))

(fn InitializeStatus
  (for _index (range 1 (* (Variables|Default|GetBoardNX) (Variables|Default|GetBoardNY)))
    (Utilities|Array|Add (Variables|Default|GetBoardStatus) false)))

(fn GetAliveNeighbours
  (params (X :type Integer) (Y :type Integer))
  (LocalVariables|SetLX X)
  (LocalVariables|SetLY Y)
  (LocalVariables|SetLNumAliveNeighbours 0)
  (Utilities|FlowControl|Sequence
    (:then_0
      (Utilities|CheckifTileActivated (LocalVariables|GetLX) (LocalVariables|GetLY) 1 1
        (:True
          (Math|Integer|IncrementInt (LocalVariables|GetLNumAliveNeighbours)))))
    (:then_1
      (Utilities|CheckifTileActivated (LocalVariables|GetLX) (LocalVariables|GetLY) 1
        (:True
          (Math|Integer|IncrementInt (LocalVariables|GetLNumAliveNeighbours)))))
    (:then_2
      (Utilities|CheckifTileActivated (LocalVariables|GetLX) (LocalVariables|GetLY) -1
        (:True
          (Math|Integer|IncrementInt (LocalVariables|GetLNumAliveNeighbours)))))
    (:then_3
      (Utilities|CheckifTileActivated (LocalVariables|GetLX) (LocalVariables|GetLY) -1 -1
        (:True
          (Math|Integer|IncrementInt (LocalVariables|GetLNumAliveNeighbours)))))
    (:then_4
      (Utilities|CheckifTileActivated (LocalVariables|GetLX) (LocalVariables|GetLY) -1
        (:True
          (Math|Integer|IncrementInt (LocalVariables|GetLNumAliveNeighbours)))))
    (:then_5
      (Utilities|CheckifTileActivated (LocalVariables|GetLX) (LocalVariables|GetLY) -1 1
        (:True
          (Math|Integer|IncrementInt (LocalVariables|GetLNumAliveNeighbours)))))
    (:then_6
      (Utilities|CheckifTileActivated (LocalVariables|GetLX) (LocalVariables|GetLY) 0 1
        (:True
          (Math|Integer|IncrementInt (LocalVariables|GetLNumAliveNeighbours)))))
    (:then_7
      (Utilities|CheckifTileActivated (LocalVariables|GetLX) (LocalVariables|GetLY) 0 -1
        (:True
          (Math|Integer|IncrementInt (LocalVariables|GetLNumAliveNeighbours)))))
    (:then_8
      (return (LocalVariables|GetLNumAliveNeighbours)))))

(fn ProcessTile
  (params (TileX :type Integer) (TileY :type Integer))
  (LocalVariables|SetLX TileX)
  (LocalVariables|SetLY TileY)
  (LocalVariables|SetLNAliveNeighbours (CallFunction|GetAliveNeighbours (LocalVariables|GetLX) (LocalVariables|GetLY)))
  (if (Utilities|Array|Get(acopy) (Variables|Default|GetBoardStatusAux) (CallFunction|GetTilePositioninArray (LocalVariables|GetLX) (LocalVariables|GetLY)))
    (if (or (< (LocalVariables|GetLNAliveNeighbours) 2) (> (LocalVariables|GetLNAliveNeighbours) 3))
      (CallFunction|DeactivateTile (LocalVariables|GetLX) (LocalVariables|GetLY)))
    (elif (== (LocalVariables|GetLNAliveNeighbours) 3)
      (CallFunction|ActivateTile (LocalVariables|GetLX) (LocalVariables|GetLY)))))

(fn ActivateTile
  (params (X :type Integer) (Y :type Integer))
  (bind _index (CallFunction|GetTilePositioninArray X Y))
  (Utilities|Array|SetArrayElem (Variables|Default|GetBoardStatusAux) _index true)
  (Default|Activate (Utilities|Array|Get(acopy) (Variables|Default|GetTiles) _index)))

(fn DeactivateTile
  (params (X :type Integer) (Y :type Integer))
  (bind _index (CallFunction|GetTilePositioninArray X Y))
  (Utilities|Array|SetArrayElem (Variables|Default|GetBoardStatusAux) _index false)
  (Default|Deactivate (Utilities|Array|Get(acopy) (Variables|Default|GetTiles) _index)))